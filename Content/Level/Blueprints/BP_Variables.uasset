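; BP_Variables counts the people in the level at BeginPlay and reports how many are in the room.
; It gathers all BP_Person actors, keeps those flagged IsPerson and uses the array length as the count.
; Branches choose plural, empty or singular wording, print it in a distinct color and store it in RoomInfo.
; Several disconnected earlier counting attempts remain in the graph, and OnRep_isPerson is empty.
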(event EventBeginPlay
  (bind _instring (Variables|Default|GetInString))
  (bind _howmanyisperson (Variables|Default|GetHowManyisPerson))
  (bind _outactors (Actor|GetAllActorsOfClass "/Game/Level/Blueprints/BP_Person.BP_Person_C"))
  (for _array_element _outactors
    (if (Variables|/Game/Level/Blueprints/BP_Person.BP_Person_C|GetisPerson? _array_element)
      (Utilities|Array|Add _howmanyisperson _array_element)
      (bind _output_get (Variables|Default|SetHow%20many%20people (Utilities|Array|Length _howmanyisperson)))))
  (if (> _output_get 1)
    (Development|PrintString (Utilities|String|Append " There are" (Utilities|String|ToString(Integer) (Variables|Default|GetHow%20many%20people)) " people in the room") true true "(R=0.334273,G=0.340625,B=0.331400,A=1.000000)" 1e+01)
    (Variables|Default|SetRoom%20Info (Utilities|String|Append " There are" (Utilities|String|ToString(Integer) (Variables|Default|GetHow%20many%20people)) " people in the room"))
    (elif (== _output_get 0)
      (Development|PrintString _instring true true "(R=0.340625,G=0.073131,B=0.154461,A=1.000000)" 1e+01)
      (Variables|Default|SetRoom%20Info _instring)
      (else
        (Development|PrintString (Utilities|String|Append " There is" (Utilities|String|ToString(Integer) (Variables|Default|GetHow%20many%20people)) " person in the room") true true "(R=0.340625,G=0.253858,B=0.047244,A=1.000000)" 1e+01)
        (Variables|Default|SetRoom%20Info (Utilities|String|Append " There is" (Utilities|String|ToString(Integer) (Variables|Default|GetHow%20many%20people)) " person in the room"))))))

(fn ConstructionScript)

(fn OnRepIsPerson)